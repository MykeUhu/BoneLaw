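; Player controller that fixes the view on the game's cine camera and controls the pace of the day/night cycle.
; On BeginPlay it blends the view to the first BP_CineCam_Game and caches the Ultra Dynamic Sky actor tagged "SkyMain".
; SetDayNightLengths writes day length, night length and time speed to the sky, initially and through two update events.
; Sunset, sunrise and hour-change bindings are present but never run.
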(event `self.ReceivePossess`
  (params (PossessedPawn :type "Pawn Object Reference")))

(event `self.ReceiveBeginPlay`
  (bind _outactors (`GameplayStatics.GetAllActorsOfClass` "/Game/Blueprints/Map/MainMap/BP_CineCam_Game.BP_CineCam_Game_C"))
  (`self.SetViewTargetWithBlend` (`|GetArrayItem` _outactors) 0.0 "VTBlend_Linear" 0.0 true)
  ; Manipulate UDS Time
  (bind _outactors_2 (`GameplayStatics.GetAllActorsOfClassWithTag` "/Game/UltraDynamicSky/Blueprints/Ultra_Dynamic_Sky.Ultra_Dynamic_Sky_C" "SkyMain"))
  (bind _output_get (set `self.UDS_Ref` (`|GetArrayItem` _outactors_2)))
  (`self.SetDayNightLengths` _output_get (`self.DayMinutes`) (`self.NightMinutes`) (`self.TimeMulti`)))

(event `SetTagForSunset`)

(event `SetTagForSunrise`)

(event `UpdateTimeMulti`
  (params (TimeMulti :type "Float (double-precision)"))
  ; Manipulate UDS Time
  (`self.SetDayNightLengths` (`self.UDS_Ref`) (`self.DayMinutes`) (`self.NightMinutes`) TimeMulti))

(event `UpdateDayNightMins`
  (params (DayMin :type "Float (double-precision)") (NightMin :type "Float (double-precision)"))
  ; Manipulate UDS Time
  (`self.SetDayNightLengths` (`self.UDS_Ref`) DayMin NightMin (`self.TimeMulti`)))

(fn `SetDayNightLengths`
  (params (UDS_Ref :type "/Game/UltraDynamicSky/Blueprints/Ultra_Dynamic_Sky Object Reference") (DayMinutes :type "Float (double-precision)") (NightMinutes :type "Float (double-precision)") (TimeMulti :type "Float (double-precision)"))
  (`/Engine/EditorBlueprintResources/StandardMacros.IsValid` UDS_Ref
    (:`Is Valid`
      (set `/Game/UltraDynamicSky/Blueprints/Ultra_Dynamic_Sky.Day Length` DayMinutes (`self.UDS_Ref`))
      (set `/Game/UltraDynamicSky/Blueprints/Ultra_Dynamic_Sky.Night Length` NightMinutes (`self.UDS_Ref`))
      (set `/Game/UltraDynamicSky/Blueprints/Ultra_Dynamic_Sky.Time Speed` TimeMulti (`self.UDS_Ref`)))))

(fn `UserConstructionScript`)